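; A Blueprint function library with helpers to get and set the real playback duration of Timelines and sequence players.
; The getters divide the timeline or sequence length by its current play rate.
; The setters compute length divided by desired duration in math expression nodes and apply it as the play rate, so playback stretches or compresses to the target time.
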(fn GetTimelineDuration
  (params (Target%20TImeline :type Timeline%20Component%20Object%20Reference))
  (return (/ (Components|Timeline|GetTimelineLength Target%20TImeline) (Components|Animation|GetPlayRate Target%20TImeline))))

(fn SetTimelineDuration
  (params (Target%20Timeline :type Timeline%20Component%20Object%20Reference) (Target%20Duration :type Float%20%28single-precision%29))
  (Components|Timeline|SetPlayRate Target%20Timeline (|(timelineLength/desiredDuration) (Components|Timeline|GetTimelineLength Target%20Timeline) Target%20Duration)))

(fn GetSequenceDuration
  (params (Sequence%20Target :type Actor%20Sequence%20Component%20Object%20Reference))
  (bind _sequenceplayer (Variables|/Script/ActorSequence.ActorSequenceComponent|GetSequencePlayer Sequence%20Target))
  (return (/ (Class|TimeManagementBlueprintLibrary|ToSeconds(QualifiedFrameTime) (Media|MediaPlayer|GetDuration _sequenceplayer)) (Components|Animation|GetPlayRate _sequenceplayer))))

(fn SetSequenceDuration
  (params (Actor%20Sequence :type Actor%20Sequence%20Component%20Object%20Reference) (Target%20Duration :type Float%20%28single-precision%29))
  (bind _sequenceplayer (Variables|/Script/ActorSequence.ActorSequenceComponent|GetSequencePlayer Actor%20Sequence))
  (Components|Timeline|SetPlayRate _sequenceplayer (|(sequenceDuration/desiredDuration) (Class|TimeManagementBlueprintLibrary|ToSeconds(QualifiedFrameTime) (Media|MediaPlayer|GetDuration _sequenceplayer)) Target%20Duration)))