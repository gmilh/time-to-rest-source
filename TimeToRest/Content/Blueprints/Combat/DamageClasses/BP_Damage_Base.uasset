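; BP_Damage_Base is a base damage class that supplies knockback and hit feedback data for combat.
; Knockback adds a fixed upward bias to the incoming direction, multiplies it by DamageImpulse, and also by base damage when ScaleKnockbackByDamage is set.
; Getters return controller feedback (camera shake, haptics) and spatial feedback (particles, sounds), leaving playback to the caller.
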(fn `Get Controller Feedback`
  (returns (`Camera Shake` :type "CameraShake Object Reference") (`Haptic Feedback` :type "HapticFeedbackEffect_Base Object Reference"))
  (return (`self.Camera Shake`) (`self.Haptic Feedback`)))

(fn `Get Knockback`
  (params (`From Direction` :type "Vector Structure") (`Base Damage` :type "Float (double-precision)"))
  (returns (Impulse :type "Vector Structure"))
  (bind _returnvalue (* (+ `From Direction` (0.0 0.0 0.4)) (`self.DamageImpulse`)))
  (return (`KismetMathLibrary.SelectVector` _returnvalue (* _returnvalue `Base Damage`) (not (`self.Scale Knockback by Damage`)))))

(fn `Get Spatial Feedback`
  (returns (`Particle Effects` :type "Array of ParticleSystem Object Reference") (`Sound Effects` :type "Array of SoundBase Object Reference"))
  (return (`self.Particle Effects`) (`self.Sound Effects`)))