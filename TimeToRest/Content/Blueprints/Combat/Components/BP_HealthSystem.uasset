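; BP_HealthSystem is a combat component that tracks an actor's current health against a maximum HitPoints value.
; On BeginPlay it fills CurrentHP to the maximum, and decrement and increment functions clamp changes between zero and that maximum.
; Each change fires the OnHPAmountUpdate dispatcher with the health percentage, which also backs the check for remaining HP.
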(event `self.ReceiveBeginPlay`
  (set `self.Current HP` (`self.Hit Points`)))

(fn `Decrement HP`
  (params (`HP Removed` :type "Float (double-precision)"))
  (returns (`Hp Remaining` :type "Float (double-precision)"))
  (set `self.Current HP` (`KismetMathLibrary.FClamp` (- (`self.Current HP`) `HP Removed`) 0.0 (`self.Hit Points`)))
  (`self.On HP Amount Update` (`self.Get HP Percent`))
  (return (`self.Current HP`)))

(fn `Get Has Remaining HP`
  (returns (`Return Value` :type Boolean))
  (return (> (`self.Get HP Percent`) 0.0)))

(fn `Get HP Percent`
  (returns (`Current HP` :type "Float (double-precision)"))
  (return (/ (`self.Current HP`) (`self.Hit Points`))))

(fn `Increment HP`
  (params (`HP Gained` :type "Float (double-precision)"))
  (set `self.Current HP` (`KismetMathLibrary.FClamp` (+ `HP Gained` (`self.Current HP`)) 0.0 (`self.Hit Points`)))
  (`self.On HP Amount Update` (`self.Get HP Percent`)))