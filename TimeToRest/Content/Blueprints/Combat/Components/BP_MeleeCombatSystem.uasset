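; Melee combat component that tracks combo progression and the current melee state.
; It serves the next attack from an overridable list, advancing the counter immediately when that attack class's defaults enable auto-advance.
; Advancing starts a combo timeout timer, while advancing past the last attack clears it and resets the combo.
; Setting the state to Idle broadcasts an attack-termination event.
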(fn `Advance Combo Counter`
  (if (!= (`self.Combo Counter`) (`KismetArrayLibrary.Array_LastIndex` (`self.Base Combo Attacks`)))
    (`/Engine/EditorBlueprintResources/StandardMacros.IncrementInt` (`self.Combo Counter`)
      (:`  `
        (bind _returnvalue (`KismetSystemLibrary.K2_SetTimerDelegate` (`|CreateDelegate` :!event `Reset Combo`) (`self.Combo Timeout`)))
        (set `self.Combo Timer` _returnvalue)))
    (else
      (`KismetSystemLibrary.K2_ClearAndInvalidateTimerHandle` (`self.Combo Timer`))
      (`self.Reset Combo`))))

(fn `Get Current State`
  (returns (`Current State` :type "/Game/Blueprints/Combat/E_MeleeState Enum"))
  (return (`self.Current State`)))

(fn `Get Next Attack in Combo`
  (returns (Success :type Boolean) (`Current Attack` :type "/Game/Blueprints/Combat/AttackClasses/BP_Attack_Base Class Reference"))
  (locals (`Attack to Return` :type "/Game/Blueprints/Combat/AttackClasses/BP_Attack_Base Class Reference"))
  ;[1 1 1] Select next attack in combo
  (bind _output_get (set `local.Attack to Return` (`|GetArrayItem` (`self.Base Combo Attacks`) (`self.Combo Counter`))))
  (if (defaults `/Game/Blueprints/Combat/Components/BP_MeleeCombatSystem` _output_get)
    (`self.Advance Combo Counter`)
    (return true (`local.Attack to Return`))
    (else
      (return true (`local.Attack to Return`)))))

(fn `Override Combo Attacks`
  (params (`Base Combo Attacks` :type "Array of /Game/Blueprints/Combat/AttackClasses/BP_Attack_Base Class Reference"))
  (set `self.Base Combo Attacks` `Base Combo Attacks`))

(fn `Reset Combo`
  (set `self.Combo Counter` 0))

(fn `Set Melee State`
  (params (`New State` :type "/Game/Blueprints/Combat/E_MeleeState Enum" :default "NewEnumerator0"))
  (bind _output_get (set `self.Current State` `New State`))
  (switch `/Game/Blueprints/Combat/E_MeleeState` _output_get
    (:`NewEnumerator0`
      (`self.On Terminate Attack`))))