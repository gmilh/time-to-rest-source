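; Actor component that picks and launches the character's grounded dodge from movement input, gated by dodge state and melee combo state.
; It chooses a back dodge, a camera-relative roll, or, when strafing or locked on, forward and side dodges.
; Capsule traces set those strafe dodges' destinations, with sides arcing around distant targets and distance scaling playback rate.
; A dispatcher passes montage and move data out, and a timed recovery state allows re-dodging.
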(event Custom|Initiate%20Dodge
  (params (Movement%20Input :type Vector%202D%20Structure))
  (bind _capsule_component (Variables|Default|GetCapsule%20Component))
  (bind _capsule_component_2 (Variables|Default|GetCapsule%20Component))
  (bind (_outradius _outhalfheight) (Components|Capsule|GetScaledCapsuleSize _capsule_component))
  (bind (_outradius_2 _outhalfheight_2) (Components|Capsule|GetScaledCapsuleSize _capsule_component_2))
  (Variables|Default|SetDodge%20Input Movement%20Input)
  (switch Utilities|FlowControl|Switch|SwitchonE_DodgeState (Variables|Default|GetCurrent%20Dodge%20State)
    (:NewEnumerator0
      _)
    (:NewEnumerator2
      (CallFunction|ResetDodgeState)))
  (if (AI|Components|NavMovement|IsMovingonGround (Variables|Default|GetCharacter%20Movement))
    (bind _current_state (Default|GetCurrentState (Variables|Default|GetMelee%20Combo)))
    (switch Utilities|FlowControl|Switch|SwitchonE_MeleeState _current_state
      (:NewEnumerator0
        _)
      (:NewEnumerator4)
      (:NewEnumerator5
        _))
    (if (and (or (== (.X (Math|Vector2D|BreakVector2D (Variables|Default|GetDodge%20Input))) 0.0) (and (<= (.X (Math|Vector2D|BreakVector2D (Variables|Default|GetDodge%20Input))) 0.0) (CallFunction|GetIsStrafing))) (== (.Y (Math|Vector2D|BreakVector2D (Variables|Default|GetDodge%20Input))) 0.0))
      ;[1 1 1] Dodge Back
      (Variables|Default|SetDodge%20In%20Use "NewEnumerator2")
      (Default|CallOnExecuteDodge :Anim%20Montage (.Value (Utilities|Map|Find (Variables|Default|GetDodge%20Animations) (Variables|Default|GetDodge%20In%20Use))) :Montage%20Play%20Rate 1.56 :Ease%20Out true :Shortest%20Rotation true)
      (Variables|Default|SetCurrent%20Dodge%20State "NewEnumerator1")
      (elif (CallFunction|GetIsStrafing)
        (if (and (> (.X (Math|Vector2D|BreakVector2D (Variables|Default|GetDodge%20Input))) 0.0) (Math|Float|NearlyEqual(Float) (.Y (Math|Vector2D|BreakVector2D (Variables|Default|GetDodge%20Input))) 0.0 0.3))
          ;[1 1 1] Dodge Forward
          (bind _outhit (Collision|CapsuleTraceByChannel (Transformation|GetActorLocation (Components|GetOwner)) (Math|Vector|SelectVector (Transformation|GetActorLocation (Default|GetLockedonActor (Variables|Default|GetLock%20On%20Component))) (+ (Transformation|GetActorLocation (Components|GetOwner)) (* (Math|Vector|SelectVector (Transformation|GetActorForwardVector (Components|GetOwner)) (Math|Vector|GetUnitDirection(Vector) (Transformation|GetActorLocation (Components|GetOwner)) (Transformation|GetActorLocation (Default|GetLockedonActor (Variables|Default|GetLock%20On%20Component)))) (Utilities|Enum|Equal(Enum) (Default|GetCurrentCameraState (Variables|Default|GetDynamic%20Camera%20Component)) "NewEnumerator5")) 3.2e+02)) (<= (Math|Vector|Distance2D(Vector) (Transformation|GetActorLocation (Components|GetOwner)) (Transformation|GetActorLocation (Default|GetLockedonActor (Variables|Default|GetLock%20On%20Component)))) 3.2e+02)) _outradius _outhalfheight "TraceTypeQuery1" true 0 "None"))
          (Variables|Default|SetDodge%20In%20Use "NewEnumerator1")
          (bind _returnvalue (Animation|GetPlayLength (.Value (Utilities|Map|Find (Variables|Default|GetDodge%20Animations) (Variables|Default|GetDodge%20In%20Use)))))
          (Default|CallOnExecuteDodge (.Value (Utilities|Map|Find (Variables|Default|GetDodge%20Animations) (Variables|Default|GetDodge%20In%20Use))) (Math|Float|MapRangeClamped (Math|Vector|Distance2D(Vector) (Math|Vector|SelectVector (+ (.Location (Collision|BreakHitResult _outhit)) (* (Math|Vector|GetUnitDirection(Vector) (.Location (Collision|BreakHitResult _outhit)) (.TraceStart (Collision|BreakHitResult _outhit))) 0.0)) (+ (* (Math|Vector|GetUnitDirection(Vector) (.TraceStart (Collision|BreakHitResult _outhit)) (.TraceEnd (Collision|BreakHitResult _outhit))) 2.6e+02) (.TraceStart (Collision|BreakHitResult _outhit))) (.bBlockingHit (Collision|BreakHitResult _outhit))) (Transformation|GetActorLocation (Components|GetOwner))) 0.0 2e+02 1.72 1.48) true (Math|Vector|SelectVector (+ (.Location (Collision|BreakHitResult _outhit)) (* (Math|Vector|GetUnitDirection(Vector) (.Location (Collision|BreakHitResult _outhit)) (.TraceStart (Collision|BreakHitResult _outhit))) 0.0)) (+ (* (Math|Vector|GetUnitDirection(Vector) (.TraceStart (Collision|BreakHitResult _outhit)) (.TraceEnd (Collision|BreakHitResult _outhit))) 2.6e+02) (.TraceStart (Collision|BreakHitResult _outhit))) (.bBlockingHit (Collision|BreakHitResult _outhit))) (Math|Rotator|MakeRotator 0.0 0.0 (.Yaw (Math|Rotator|BreakRotator (Math|Rotator|FindLookatRotation (Math|Vector|SelectVector (+ (.Location (Collision|BreakHitResult _outhit)) (* (Math|Vector|GetUnitDirection(Vector) (.Location (Collision|BreakHitResult _outhit)) (.TraceStart (Collision|BreakHitResult _outhit))) 0.0)) (+ (* (Math|Vector|GetUnitDirection(Vector) (.TraceStart (Collision|BreakHitResult _outhit)) (.TraceEnd (Collision|BreakHitResult _outhit))) 2.6e+02) (.TraceStart (Collision|BreakHitResult _outhit))) (.bBlockingHit (Collision|BreakHitResult _outhit))) (Transformation|GetActorLocation (Default|GetLockedonActor (Variables|Default|GetLock%20On%20Component))))))) false true (* (/ _returnvalue (Math|Float|MapRangeClamped (Math|Vector|Distance2D(Vector) (Math|Vector|SelectVector (+ (.Location (Collision|BreakHitResult _outhit)) (* (Math|Vector|GetUnitDirection(Vector) (.Location (Collision|BreakHitResult _outhit)) (.TraceStart (Collision|BreakHitResult _outhit))) 0.0)) (+ (* (Math|Vector|GetUnitDirection(Vector) (.TraceStart (Collision|BreakHitResult _outhit)) (.TraceEnd (Collision|BreakHitResult _outhit))) 2.6e+02) (.TraceStart (Collision|BreakHitResult _outhit))) (.bBlockingHit (Collision|BreakHitResult _outhit))) (Transformation|GetActorLocation (Components|GetOwner))) 0.0 2e+02 1.72 1.48)) 0.62) false)
          (Variables|Default|SetCurrent%20Dodge%20State "NewEnumerator1")
          (else
            ;[1 1 1] Side Dodge
            (bind _outhit_2 (Collision|CapsuleTraceByChannel (Transformation|GetActorLocation (Components|GetOwner)) (Math|Vector|SelectVector (+ (Transformation|GetActorLocation (Default|GetLockedonActor (Variables|Default|GetLock%20On%20Component))) (* (Math|Vector|GetForwardVector (Math|Rotator|CombineRotators (Math|Rotator|FindLookatRotation (Transformation|GetActorLocation (Default|GetLockedonActor (Variables|Default|GetLock%20On%20Component))) (Transformation|GetActorLocation (Components|GetOwner))) (Math|Rotator|MakeRotator 0.0 0.0 (* (Math|Integer|SelectInt -1 1 (>= (.Y (Math|Vector2D|BreakVector2D (Variables|Default|GetDodge%20Input))) 0.0)) (|((constAngle*constDistance)/DistanceGiven) 115.0 1.5e+02 (Math|Vector|Distance2D(Vector) (Transformation|GetActorLocation (Default|GetLockedonActor (Variables|Default|GetLock%20On%20Component))) (Transformation|GetActorLocation (Components|GetOwner)))))))) (Math|Vector|Distance2D(Vector) (Transformation|GetActorLocation (Default|GetLockedonActor (Variables|Default|GetLock%20On%20Component))) (Transformation|GetActorLocation (Components|GetOwner))))) (+ (* (* (Transformation|GetActorRightVector (Components|GetOwner)) (Math|Float|SelectFloat 1.0 -1.0 (>= (.Y (Math|Vector2D|BreakVector2D (Variables|Default|GetDodge%20Input))) 0.0))) 2.8e+02) (Transformation|GetActorLocation (Components|GetOwner))) (and (>= (Math|Vector|Distance2D(Vector) (Transformation|GetActorLocation (Default|GetLockedonActor (Variables|Default|GetLock%20On%20Component))) (Transformation|GetActorLocation (Components|GetOwner))) 1.8e+02) (Utilities|Enum|NotEqual(Enum) (Default|GetCurrentCameraState (Variables|Default|GetDynamic%20Camera%20Component)) "NewEnumerator5"))) _outradius_2 _outhalfheight_2 "TraceTypeQuery2" true 0 "ForDuration"))
            (Variables|Default|SetDodge%20In%20Use (select (>= (.Y (Math|Vector2D|BreakVector2D (Variables|Default|GetDodge%20Input))) 0.0) "NewEnumerator4" "NewEnumerator3"))
            (bind _returnvalue_2 (Animation|GetPlayLength (.Value (Utilities|Map|Find (Variables|Default|GetDodge%20Animations) (Variables|Default|GetDodge%20In%20Use)))))
            (Default|CallOnExecuteDodge (.Value (Utilities|Map|Find (Variables|Default|GetDodge%20Animations) (Variables|Default|GetDodge%20In%20Use))) (Math|Float|MapRangeClamped (Math|Vector|Distance2D(Vector) (Math|Vector|SelectVector (.Location (Collision|BreakHitResult _outhit_2)) (.TraceEnd (Collision|BreakHitResult _outhit_2)) (.bBlockingHit (Collision|BreakHitResult _outhit_2))) (Transformation|GetActorLocation (Components|GetOwner))) 0.0 2e+02 1.72 1.48) true (Math|Vector|SelectVector (.Location (Collision|BreakHitResult _outhit_2)) (.TraceEnd (Collision|BreakHitResult _outhit_2)) (.bBlockingHit (Collision|BreakHitResult _outhit_2))) (Transformation|GetActorRotation (Components|GetOwner)) false true (* (/ _returnvalue_2 (Math|Float|MapRangeClamped (Math|Vector|Distance2D(Vector) (Math|Vector|SelectVector (.Location (Collision|BreakHitResult _outhit_2)) (.TraceEnd (Collision|BreakHitResult _outhit_2)) (.bBlockingHit (Collision|BreakHitResult _outhit_2))) (Transformation|GetActorLocation (Components|GetOwner))) 0.0 2e+02 1.72 1.48)) 0.46) false)
            (Variables|Default|SetCurrent%20Dodge%20State "NewEnumerator1")))
        (else
          ;[1 1 1] Dodge Roll
          (Variables|Default|SetDodge%20In%20Use "NewEnumerator5")
          (Default|CallOnExecuteDodge (.Value (Utilities|Map|Find (Variables|Default|GetDodge%20Animations) (Variables|Default|GetDodge%20In%20Use))) 1.0 true (Transformation|GetActorLocation (Components|GetOwner)) (CallFunction|GetDodgeRotation) true false (Math|Float|MapRangeClamped (Math|Float|Absolute(Float) (.Yaw (Math|Rotator|BreakRotator (Math|Rotator|Delta(Rotator) (Transformation|GetActorRotation (Components|GetOwner)) (CallFunction|GetDodgeRotation))))) 2e+01 1.8e+02 0.04 0.18) true)
          (Variables|Default|SetCurrent%20Dodge%20State "NewEnumerator1"))))))

(event EventBeginPlay
  ;[1 1 1] BEGIN PLAY
  (CallFunction|InitComponents))

(fn GetIsStrafing
  (return (or (Utilities|Enum|Equal(Enum) (Default|GetCurrentCameraState (Variables|Default|GetDynamic%20Camera%20Component)) "NewEnumerator5") (Default|GetLockonState (Variables|Default|GetLock%20On%20Component)))))

(fn GetDodgeRotation
  (bind _returnvalue (Components|GetOwner))
  (bind _dodge_input (Variables|Default|GetDodge%20Input))
  (bind (_x _y) (Math|Vector2D|BreakVector2D _dodge_input))
  (bind _instigator (Variables|/Script/Engine.Actor|GetInstigator _returnvalue))
  (bind _returnvalue_2 (Pawn|GetControlRotation _instigator :!class /Script/Engine.Pawn))
  (bind _yaw (Math|Rotator|BreakRotator _returnvalue_2))
  (bind _returnvalue_3 (Math|Rotator|MakeRotator 0.0 0.0 _yaw))
  (return (Math|Rotator|SelectRotator (Transformation|GetActorRotation (Components|GetOwner)) (Math|Conversions|RotationFromXVector (+ (* (Math|Vector|GetForwardVector _returnvalue_3) _x) (* (Math|Vector|GetRightVector _returnvalue_3) _y))) (Math|Vector|Equal(Vector) :A (Variables|Default|GetDodge%20Input)))))

(fn SetDodgeState
  (params (New%20State :type E_DodgeState%20Enum :default "NewEnumerator0"))
  (Variables|Default|SetCurrent%20Dodge%20State New%20State))

(fn GetCurrentState
  (return (Variables|Default|GetCurrent%20Dodge%20State) (Variables|Default|GetDodge%20In%20Use)))

(fn InitComponents
  (Variables|Default|SetLock%20On%20Component (Actor|GetComponentbyClass (Components|GetOwner) "/Game/Blueprints/Camera/BP_LockOnSystem.BP_LockOnSystem_C"))
  (Variables|Default|SetCharacter%20Movement (Actor|GetComponentbyClass (Components|GetOwner) "/Script/Engine.CharacterMovementComponent"))
  (Variables|Default|SetCapsule%20Component (Actor|GetComponentbyClass (Components|GetOwner) "/Script/Engine.CapsuleComponent"))
  (Variables|Default|SetDynamic%20Camera%20Component (Actor|GetComponentbyClass (Components|GetOwner) "/Game/Blueprints/Camera/BP_DynamicCameraSystem.BP_DynamicCameraSystem_C"))
  (Variables|Default|SetMelee%20Combo (Actor|GetComponentbyClass (Components|GetOwner) "/Game/Blueprints/Combat/Components/BP_MeleeCombatSystem.BP_MeleeCombatSystem_C")))

(fn EnterRecoveryPeriod
  (Variables|Default|SetCurrent%20Dodge%20State "NewEnumerator2")
  (bind _returnvalue (Utilities|Time|SetTimerbyEvent (EventDispatchers|CreateEvent :!event ResetDodgeState) (Variables|Default|GetRecovery%20Duration)))
  (Variables|Default|SetRecovery%20Timer _returnvalue)
  (Default|CallOnEnterRecoveryState (Variables|Default|GetDodge%20In%20Use)))

(fn ResetDodgeState
  (Variables|Default|SetCurrent%20Dodge%20State "NewEnumerator0")
  (Utilities|Time|ClearandInvalidateTimerbyHandle (Variables|Default|GetRecovery%20Timer)))