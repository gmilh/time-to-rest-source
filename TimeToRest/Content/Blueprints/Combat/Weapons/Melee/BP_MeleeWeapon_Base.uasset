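; Base melee weapon actor that applies damage to actors overlapping its Box while an attack's damage window is open, acting on behalf of its parent actor.
; Initiate and terminate events open and close the window, checking current overlaps at the start and new ones through begin overlap.
; Each actor is hit once per window.
; Targets with controllers are damaged only across the player/non-player divide, while uncontrolled actors are always eligible.
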(event `/Game/Blueprints/Combat/Weapons/Melee/BPI_MeleeWeapon.Initiate Dealing Damage`
  (params (`Damage Data` :type "/Game/Blueprints/Combat/DamageClasses/S_DamageData Structure"))
  ;[1 1 1] Begin Dealing Damage to Overlapping Actors
  (set `self.Current Attack Damage` `Damage Data`)
  (set `self.Dealing Damage` true)
  (for _array_element (`PrimitiveComponent.GetOverlappingActors` (`self.Box`) "/Script/Engine.Actor")
    (`self.Try Damaging Actor` _array_element)))

(event `self.Box.OnComponentBeginOverlap`
  (params (OverlappedComponent :type "PrimitiveComponent Object Reference") (OtherActor :type "Actor Object Reference") (OtherComp :type "PrimitiveComponent Object Reference") (OtherBodyIndex :type Integer) (bFromSweep :type Boolean) (SweepResult :type "HitResult Structure (by ref)"))
  (if (`self.Dealing Damage`)
    (`self.Try Damaging Actor` OtherActor)))

(event `/Game/Blueprints/Combat/Weapons/Melee/BPI_MeleeWeapon.Terminate Dealing Damage`
  ;[1 1 1] Stop Dealing Damage
  (set `self.Dealing Damage` false)
  (`KismetArrayLibrary.Array_Clear` (`self.Actors Damaged`))
  (set `self.Current Attack Damage` (struct)))

(fn `Try Damaging Actor`
  (params (Actor :type "Actor Object Reference"))
  (locals (`Actor Parameter` :type "Actor Object Reference"))
  (bind (_basedamage _damagetype) (break `/Game/Blueprints/Combat/DamageClasses/S_DamageData` (`self.Current Attack Damage`)))
  (bind _returnvalue (`self.GetInstigatorController` (`local.Actor Parameter`)))
  (set `local.Actor Parameter` Actor)
  (`/Engine/EditorBlueprintResources/StandardMacros.IsValid` _returnvalue
    (:`Is Valid`
      (if (!= (`Controller.IsPlayerController` (`self.GetInstigatorController` (`self.GetParentActor`))) (`Controller.IsPlayerController` _returnvalue))
        (if (and (not (`KismetArrayLibrary.Array_Contains` (`self.Actors Damaged`) (`local.Actor Parameter`))) (!= (`local.Actor Parameter`) (`self.GetParentActor`))) :!label _label
          (`KismetArrayLibrary.Array_Add` (`self.Actors Damaged`) (`local.Actor Parameter`))
          (`GameplayStatics.ApplyDamage` (`local.Actor Parameter`) _basedamage (`self.GetInstigatorController` (`self.GetParentActor`)) self _damagetype))))
    (:`Is Not Valid`
      (goto _label))))

(fn `UserConstructionScript`)