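; Thrown melee weapon projectile that shows the configured weapon class as a child actor and can be called back to its thrower.
; Static world hits stop flight and spin; CallBack disables projectile movement, restarts spin and starts the return.
; Tick moves it toward the instigator, box-tracing with a growing Z offset around obstacles and teleporting it closer when too far.
; Overlapping the instigator while returning destroys it; debug prints and traces remain active.
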(event Collision|EventHit
  (params (MyComp :type Primitive%20Component%20Object%20Reference) (Other :type Actor%20Object%20Reference) (OtherComp :type Primitive%20Component%20Object%20Reference) (bSelfMoved :type Boolean) (HitLocation :type Vector :default "0, 0, 0") (HitNormal :type Vector :default "0, 0, 0") (NormalImpulse :type Vector :default "0, 0, 0") (Hit :type Hit%20Result%20Structure%20%28by%20ref%29))
  (|CallParentFunction MyComp Other OtherComp bSelfMoved HitLocation HitNormal NormalImpulse Hit)
  (if (Utilities|Enum|Equal(Enum) (Collision|GetCollisionObjectType OtherComp) "ECC_WorldStatic")
    (|CallParentFunction)
    (Components|Activation|Deactivate (Variables|Default|GetRotatingMovement))))

(event EventEnablePawnCollision)

(event EventTick
  (params (DeltaSeconds :type Float%20%28single-precision%29))
  (bind _returnvalue (Game|GetInstigator))
  (bind _returnvalue_2 (Game|GetInstigator))
  (bind _returnvalue_3 (Transformation|GetActorLocation))
  (bind _returnvalue_4 (Transformation|GetActorLocation _returnvalue))
  (bind _returnvalue_5 (Transformation|GetActorLocation _returnvalue_2))
  (bind _returnvalue_6 (Math|Vector|Distance(Vector) _returnvalue_5 _returnvalue_3))
  (if (Variables|Default|GetReturning)
    (if (>= _returnvalue_6 1.8e+03)
      (Transformation|SetActorLocation (+ _returnvalue_4 (* (Math|Vector|GetUnitDirection(Vector) _returnvalue_4 (Transformation|GetActorLocation)) 1.6e+03)) false true)
      (else
        (if (<= (Variables|Default|GetCurrent%20Z%20Offset) (Variables|Default|GetMax%20Z%20Offset)) :!label _label
          (bind _outhit (Class|KismetSystemLibrary|BoxTraceSingleforObjects (Transformation|GetActorLocation) (+ (Transformation|GetActorLocation (Game|GetInstigator)) (Math|Vector|MakeVector 0.0 0.0 (Math|Float|SelectFloat (Variables|Default|GetCurrent%20Z%20Offset) (* -1 (Variables|Default|GetCurrent%20Z%20Offset)) (stale _isa)))) (Math|Vector|MakeVector 1.0 0.0 4e+01) "0, 0, 0" (Utilities|Array|MakeArray "ObjectTypeQuery1" "ObjectTypeQuery4" "ObjectTypeQuery6" "ObjectTypeQuery5") false 0 "ForOneFrame" true))
          (if (or (not (.bBlockingHit (Collision|BreakHitResult _outhit))) (== (.HitActor (Collision|BreakHitResult _outhit)) (Game|GetInstigator)))
            _
            (else
              (Variables|Default|SetCurrent%20Z%20Offset (+ (Variables|Default|GetCurrent%20Z%20Offset) 1.0))
              (goto _label))))
        (Development|PrintString (Utilities|String|ToString(Float) (Variables|Default|GetCurrent%20Z%20Offset)))
        (Transformation|SetActorLocation (Math|Interpolation|VInterptoConstant (Transformation|GetActorLocation) (+ (Transformation|GetActorLocation (Game|GetInstigator)) (Math|Vector|MakeVector 0.0 0.0 (* (Math|Float|SelectFloat 0.0 (Variables|Default|GetCurrent%20Z%20Offset) (== (Variables|Default|GetCurrent%20Z%20Offset) 0.0)) 2e+01))) (Utilities|Time|GetWorldDeltaSeconds) 1.28e+03) true false)))
    (else
      (Development|PrintString (Utilities|String|ToString(Float) _returnvalue_6)))))

(event EventCallBack
  (Components|Activation|Deactivate (Variables|Default|GetProjectileMovement))
  (Components|Activation|Activate (Variables|Default|GetRotatingMovement) true)
  (Variables|Default|SetReturning true)
  (CallFunction|ResetHit))

(event EventArrestProjectileMovement
  ;[1 1 1] Override functions that should be disabled
)

(event Collision|EventActorBeginOverlap
  (params (OtherActor :type Actor%20Object%20Reference))
  (if (and (Variables|Default|GetReturning) (== OtherActor (Game|GetInstigator)))
    (Actor|DestroyActor)))

(fn ConstructionScript
  (|CallParentFunction)
  (ChildActorComponent|SetChildActorClass (Variables|Default|GetMelee%20Weapon) (Variables|Default|GetWeapon%20Class)))