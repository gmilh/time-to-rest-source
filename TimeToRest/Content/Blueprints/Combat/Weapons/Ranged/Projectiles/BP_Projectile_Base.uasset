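; Base combat projectile that applies point damage to pawns other than its instigator, crediting the instigator's controller.
; Pawn overlaps and hits both feed HandleHit, where a DoOnce, resettable through ResetHit, stops movement, disables rotation-follows-velocity and sets gravity before applying damage.
; Overlap detection covers pawns while they are non-blocking near the shooter.
; EnablePawnCollision would block pawns once clear of the instigator, but its delayed call is disconnected.
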(event `self.Collision.OnComponentBeginOverlap`
  (params (OverlappedComponent :type "PrimitiveComponent Object Reference") (OtherActor :type "Actor Object Reference") (OtherComp :type "PrimitiveComponent Object Reference") (OtherBodyIndex :type Integer) (bFromSweep :type Boolean) (SweepResult :type "HitResult Structure (by ref)"))
  ;[1 1 1] By default, the projectile will not Block pawns, to avoid issues if instatiate next to the shooter
  ;;[1 1 1] Catch code if projectile hits opponent while overlapping with its shooter
  (if (and (!= OtherActor (`self.GetInstigator`)) (`|EnumEquality` (`PrimitiveComponent.GetCollisionObjectType` OtherComp) "ECC_Pawn"))
    (`self.Handle Hit` SweepResult)))

(event `self.ReceiveActorEndOverlap`
  (params (OtherActor :type "Actor Object Reference"))
  ;[1 1 1] By default, the projectile will not Block pawns, to avoid issues if instatiate next to the shooter
  ;;[1 1 1] As soon as projectile stops overlapping its instigator,
  ;; pawns will start to be blocked
  (if (== OtherActor (`self.GetInstigator`))
    _))

(event `self.ReceiveHit`
  (params (MyComp :type "PrimitiveComponent Object Reference") (Other :type "Actor Object Reference") (OtherComp :type "PrimitiveComponent Object Reference") (bSelfMoved :type Boolean) (HitLocation :type "Vector Structure") (HitNormal :type "Vector Structure") (NormalImpulse :type "Vector Structure") (Hit :type "HitResult Structure (by ref)"))
  (if (!= Other (`self.GetInstigator`))
    (if (`|EnumEquality` (`PrimitiveComponent.GetCollisionObjectType` OtherComp) "ECC_Pawn")
      (`self.Handle Hit` Hit))))

(event `Handle Hit`
  (params (`Hit Data` :type "HitResult Structure"))
  (bind (_bblockinghit _binitialoverlap _time _distance _location _impactpoint _normal _impactnormal _physmat _hitactor _hitcomponent _hitbonename _hititem _faceindex _tracestart) (`GameplayStatics.BreakHitResult` `Hit Data`))
  (`/Engine/EditorBlueprintResources/StandardMacros.DoOnce` false :!label _label
    (:`Completed`
      (`self.Arrest Projectile Movement`)
      (`GameplayStatics.ApplyPointDamage` _hitactor 2.0 (`KismetMathLibrary.GetDirectionUnitVector` _tracestart _impactpoint) `Hit Data` (`self.GetInstigatorController`) self))))

(event `Reset Hit`
  (goto _label :!via `Reset`))

(fn `Arrest Projectile Movement`
  (set `ProjectileMovementComponent.bRotationFollowsVelocity` false (`self.ProjectileMovement`))
  (set `ProjectileMovementComponent.ProjectileGravityScale` 1.4 (`self.ProjectileMovement`))
  (`MovementComponent.StopMovementImmediately` (`self.ProjectileMovement`)))

(fn `Enable Pawn Collision`
  (if (not (`KismetArrayLibrary.Array_Contains` (`PrimitiveComponent.GetOverlappingActors` (`self.Collision`) "/Script/Engine.Character") (`self.GetInstigator`)))
    (`PrimitiveComponent.SetCollisionResponseToChannel` (`self.Collision`) "ECC_Pawn" "ECR_Block")))

(fn `UserConstructionScript`)