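; Actor component that provides target lock-on, steering the owner's controller rotation toward the locked target every tick.
; Lock-on picks the BPI_LockOnTarget actor best aligned with the view within range, notifies it, and re-acquires when it is destroyed.
; Directional input cycles targets on a cooldown, favoring view alignment and very close enemies.
; Pitch tracking adapts to one BP_DynamicCameraSystem state, apparently Aiming.
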(event `self.ReceiveBeginPlay`
  (`self.Init Components`))

(event `self.ReceiveTick`
  (params (DeltaSeconds :type "Float (single-precision)"))
  (`self.Update Camera Rotation`))

(event `Target Destroyed`
  (params (DestroyedActor :type "Actor Object Reference"))
  (`self.Enter Lock On`))

(fn `Cycle Locked On Target`
  (params (`Input Dir` :type "Vector2D Structure"))
  (locals (`Cycle Dir` :type "Vector2D Structure") (`Available Targetrs` :type "Array of Actor Object Reference") (`Next Target` :type "Actor Object Reference"))
  (bind _returnvalue (`self.GetOwner`))
  (bind _returnvalue_2 (`self.GetOwner`))
  (bind _returnvalue_3 (`Actor.K2_GetActorLocation` _returnvalue_2))
  (bind _returnvalue_4 (`SceneComponent.K2_GetComponentLocation` (`self.Camera Component`)))
  (bind (_x _y) (`KismetMathLibrary.BreakVector2D` (`local.Cycle Dir`)))
  (bind _returnvalue_5 (`SceneComponent.K2_GetComponentLocation` (`self.Camera Component`)))
  (bind _returnvalue_6 (`Actor.K2_GetActorLocation` (`local.Next Target`)))
  (bind _returnvalue_7 (`KismetMathLibrary.Vector_Distance2D` (`Actor.K2_GetActorLocation` _returnvalue) _returnvalue_6))
  (bind _returnvalue_8 (`KismetMathLibrary.Dot_VectorVector` (`KismetMathLibrary.GetDirectionUnitVector` _returnvalue_4 _returnvalue_6) (`KismetMathLibrary.GetForwardVector` (`Pawn.GetControlRotation` (`Actor.Instigator` _returnvalue)))))
  (bind _output_get (set `local.Cycle Dir` `Input Dir`))
  (bind _return_value (message `/Game/Blueprints/Game/BPI_InputDeviceData.Get Using Gamepad` (`GameplayStatics.GetGameInstance`)))
  (bind (_x_2 _y_2) (`KismetMathLibrary.BreakVector2D` _output_get))
  (bind _returnvalue_9 (`KismetMathLibrary.SelectFloat` 0.32 1.0 _return_value))
  (if (or (>= (`KismetMathLibrary.Abs` _x_2) _returnvalue_9) (>= (`KismetMathLibrary.Abs` _y_2) _returnvalue_9))
    (if (`self.Can Cycle Targets`)
      (set `self.Can Cycle Targets` false)
      (bind _returnvalue_10 (`KismetSystemLibrary.K2_SetTimerDelegate` (`|CreateDelegate` :!event `Enable Target Cycling`) 0.32))
      (set `self.Cycling Cooldown` _returnvalue_10)
      (bind _outactors (`GameplayStatics.GetAllActorsWithInterface` "/Game/Blueprints/Combat/Interfaces/BPI_LockOnTarget.BPI_LockOnTarget_C"))
      (for _array_element _outactors
        (bind _returnvalue_11 (`Actor.K2_GetActorLocation` _array_element))
        (if (and (<= (`KismetMathLibrary.Vector_Distance2D` _returnvalue_11 _returnvalue_3) 3200.0) (>= (`KismetMathLibrary.Dot_VectorVector` (`KismetMathLibrary.GetDirectionUnitVector` _returnvalue_3 _returnvalue_11) (`KismetMathLibrary.GetForwardVector` (`Pawn.GetControlRotation` (`Actor.Instigator` _returnvalue_2)))) -0.3))
          (`KismetArrayLibrary.Array_Add` (`local.Available Targetrs`) _array_element)))
      (`KismetArrayLibrary.Array_RemoveItem` (`local.Available Targetrs`) (`self.Current Lock On Target`))
      (for _array_element_2 (`local.Available Targetrs`)
        (bind _returnvalue_12 (`KismetMathLibrary.NormalizedDeltaRotator` (`KismetMathLibrary.FindLookAtRotation` _returnvalue_5 (`Actor.K2_GetActorLocation` _array_element_2)) (`KismetMathLibrary.FindLookAtRotation` _returnvalue_5 (`Actor.K2_GetActorLocation` (`self.Current Lock On Target`)))))
        (if (or (== _returnvalue_12 (struct) :`ErrorTolerance` 2.0) (select `bool` (>= (`KismetMathLibrary.Abs` _x) (`KismetMathLibrary.Abs` _y)) :`false` (== (>= (.pitch _returnvalue_12) 0.0) (>= _y 0.0)) :`true` (== (>= (.yaw _returnvalue_12) 0.0) (>= _x 0.0))))
          (`local.Next Target`
            (:`then`
              (bind _returnvalue_13 (`Actor.K2_GetActorLocation` _array_element_2))
              (bind _returnvalue_14 (`KismetMathLibrary.Dot_VectorVector` (`KismetMathLibrary.GetDirectionUnitVector` _returnvalue_4 _returnvalue_13) (`KismetMathLibrary.GetForwardVector` (`Pawn.GetControlRotation` (`Actor.Instigator` _returnvalue)))))
              (bind _returnvalue_15 (`KismetMathLibrary.Vector_Distance2D` (`Actor.K2_GetActorLocation` _returnvalue) _returnvalue_13))
              (bind _returnvalue_16 (< _returnvalue_15 _returnvalue_7))
              (if (or (and (or (>= _returnvalue_14 _returnvalue_8) (and (`KismetMathLibrary.NearlyEqual_FloatFloat` _returnvalue_14 _returnvalue_8 0.15) _returnvalue_16 (<= (`.Y` (`KismetMathLibrary.BreakVector2D` (`local.Cycle Dir`))) 0.0))) (not (<= _returnvalue_7 280.0))) (and (<= _returnvalue_15 280.0) _returnvalue_16))
                (set `local.Next Target` _array_element_2 :!label _label)))
            (:`else`
              (goto _label)))))
      (`local.Next Target`
        (:`then`
          ;[1 1 1] Set new lock on target
          (message `/Game/Blueprints/Combat/Interfaces/BPI_LockOnTarget.Set Is Targeted` (`self.Current Lock On Target`) false)
          (remove `Actor.OnDestroyed` (`self.Current Lock On Target`) (`|CreateDelegate` :!event `Target Destroyed`))
          (set `self.Current Lock On Target` (`local.Next Target`))
          (message `/Game/Blueprints/Combat/Interfaces/BPI_LockOnTarget.Set Is Targeted` (`self.Current Lock On Target`) true)
          (add `Actor.OnDestroyed` (`self.Current Lock On Target`) (`|CreateDelegate` :!event `Target Destroyed`)))
        (:`else`)))
    (elif _return_value
      (`self.Enable Target Cycling`))))

(fn `Enable Target Cycling`
  (set `self.Can Cycle Targets` true)
  (`KismetSystemLibrary.K2_ClearAndInvalidateTimerHandle` (`self.Cycling Cooldown`)))

(fn `End Lock On`
  (message `/Game/Blueprints/Combat/Interfaces/BPI_LockOnTarget.Set Is Targeted` (`self.Current Lock On Target`) false)
  (set `self.Current Lock On Target` null)
  (`self.On LockOn State Change` false))

(fn `Enter Lock On`
  (locals (`Available Targetrs` :type "Array of Actor Object Reference"))
  (bind _returnvalue (`self.GetOwner`))
  (bind _returnvalue_2 (`self.GetOwner`))
  (bind _returnvalue_3 (`Actor.K2_GetActorLocation` _returnvalue_2))
  (bind _current_lock_on_target (`self.Current Lock On Target`)
    (:`then`
      (message `/Game/Blueprints/Combat/Interfaces/BPI_LockOnTarget.Set Is Targeted` _current_lock_on_target false))
    (:`else`
      _))
  (bind _outactors (`GameplayStatics.GetAllActorsWithInterface` "/Game/Blueprints/Combat/Interfaces/BPI_LockOnTarget.BPI_LockOnTarget_C"))
  (for _array_element _outactors
    (bind _returnvalue_4 (`Actor.K2_GetActorLocation` _array_element))
    (if (and (<= (`KismetMathLibrary.Vector_Distance2D` _returnvalue_4 _returnvalue_3) 3200.0) (>= (`KismetMathLibrary.Dot_VectorVector` (`KismetMathLibrary.GetDirectionUnitVector` _returnvalue_3 _returnvalue_4) (`KismetMathLibrary.GetForwardVector` (`Pawn.GetControlRotation` (`Actor.Instigator` _returnvalue_2)))) -0.3))
      (`KismetArrayLibrary.Array_Add` (`local.Available Targetrs`) _array_element)))
  (for (_array_element_2 _array_index) (`local.Available Targetrs`)
    (switch `int` _array_index
      (:`Default`
        (if (> (`KismetMathLibrary.Dot_VectorVector` (`KismetMathLibrary.GetDirectionUnitVector` (`Actor.K2_GetActorLocation` _returnvalue) (`Actor.K2_GetActorLocation` _array_element_2)) (`KismetMathLibrary.GetForwardVector` (`Pawn.GetControlRotation` (`Actor.Instigator` _returnvalue)))) (`KismetMathLibrary.Dot_VectorVector` (`KismetMathLibrary.GetDirectionUnitVector` (`Actor.K2_GetActorLocation` _returnvalue) (`Actor.K2_GetActorLocation` (`self.Current Lock On Target`))) (`KismetMathLibrary.GetForwardVector` (`Pawn.GetControlRotation` (`Actor.Instigator` _returnvalue)))))
          (set `self.Current Lock On Target` _array_element_2 :!label _label)))
      (:`0`
        (goto _label))))
  (message `/Game/Blueprints/Combat/Interfaces/BPI_LockOnTarget.Set Is Targeted` (`self.Current Lock On Target`) true)
  (add `Actor.OnDestroyed` (`self.Current Lock On Target`) (`|CreateDelegate` :!event `Target Destroyed`))
  (`self.On LockOn State Change` true))

(fn `Get Lock On State`
  (returns (`Lock On Active` :type Boolean))
  (bind _returnvalue (`KismetSystemLibrary.IsValid` (`self.Current Lock On Target`)))
  (bind _dynamic_camera_component (`self.Dynamic Camera Component`)
    (:`then`
      (return _returnvalue))
    (:`else`
      (return _returnvalue))))

(fn `Get Locked On Actor`
  (returns (`Current Lock On Target` :type "Actor Object Reference"))
  (return (`self.Current Lock On Target`)))

(fn `Init Components`
  (bind _returnvalue (`Actor.GetComponentByClass` (`self.GetOwner`) "/Game/Blueprints/Camera/BP_DynamicCameraSystem.BP_DynamicCameraSystem_C"))
  (set `self.Camera Component` (`Actor.GetComponentByClass` (`self.GetOwner`) "/Script/Engine.CameraComponent"))
  ;[1 1 1] Stores a references to the owning actor dynamic camera component if it have an Aiming configuration, as both that camera state and the lock on component
  ; will affect the owning actor rotation behaviour
  (`/Engine/EditorBlueprintResources/StandardMacros.IsValid` _returnvalue
    (:`Is Valid`
      (if (`BlueprintMapLibrary.Map_Contains` (`/Game/Blueprints/Camera/BP_DynamicCameraSystem.Camera Configurations` _returnvalue) "NewEnumerator5")
        (set `self.Dynamic Camera Component` _returnvalue)))))

(fn `Set Lock On Target`
  (params (`New LockOn Target` :type "Actor Object Reference")))

(fn `Toggle Lock On`
  (if (`self.Get Lock On State`)
    (`self.End Lock On`)
    (else
      (`self.Enter Lock On`))))

(fn `Update Camera Rotation`
  (bind _pitch (.pitch (`KismetMathLibrary.FindLookAtRotation` (`Actor.K2_GetActorLocation` (`self.GetOwner`)) (`Actor.K2_GetActorLocation` (`self.Get Locked On Actor`)))))
  (bind _returnvalue (* (`KismetMathLibrary.NormalizeAxis` (.pitch (`KismetMathLibrary.NormalizedDeltaRotator` (`KismetMathLibrary.MakeRotator` (.roll (`KismetMathLibrary.FindLookAtRotation` (`Actor.K2_GetActorLocation` (`self.GetOwner`)) (`Actor.K2_GetActorLocation` (`self.Get Locked On Actor`)))) (`KismetMathLibrary.SelectFloat` _pitch (`KismetMathLibrary.FClamp` (* _pitch 1.65) -45.0 -15.0) (`|EnumEquality` (`/Game/Blueprints/Camera/BP_DynamicCameraSystem.Get Current Camera State` (`self.Dynamic Camera Component`)) "NewEnumerator5")) (.yaw (`KismetMathLibrary.FindLookAtRotation` (`Actor.K2_GetActorLocation` (`self.GetOwner`)) (`Actor.K2_GetActorLocation` (`self.Get Locked On Actor`))))) (`Pawn.GetControlRotation` (`Actor.Instigator` (`self.GetOwner`)))))) (`GameplayStatics.GetWorldDeltaSeconds`)))
  (if (`self.Get Lock On State`)
    (`Pawn.AddControllerPitchInput` (`Actor.Instigator` (`self.GetOwner`)) (`KismetMathLibrary.SelectFloat` _returnvalue (`KismetMathLibrary.FClamp` _returnvalue -1.0) (`|EnumEquality` (`/Game/Blueprints/Camera/BP_DynamicCameraSystem.Get Current Camera State` (`self.Dynamic Camera Component`)) "NewEnumerator5")))
    (`Pawn.AddControllerYawInput` (`Actor.Instigator` (`self.GetOwner`)) (`KismetMathLibrary.FClamp` (* (`KismetMathLibrary.NormalizeAxis` (.yaw (`KismetMathLibrary.NormalizedDeltaRotator` (`KismetMathLibrary.MakeRotator` (.roll (`KismetMathLibrary.FindLookAtRotation` (`Actor.K2_GetActorLocation` (`self.GetOwner`)) (`Actor.K2_GetActorLocation` (`self.Get Locked On Actor`)))) (`KismetMathLibrary.SelectFloat` _pitch (`KismetMathLibrary.FClamp` (* _pitch 1.65) -45.0 -15.0) (`|EnumEquality` (`/Game/Blueprints/Camera/BP_DynamicCameraSystem.Get Current Camera State` (`self.Dynamic Camera Component`)) "NewEnumerator5")) (.yaw (`KismetMathLibrary.FindLookAtRotation` (`Actor.K2_GetActorLocation` (`self.GetOwner`)) (`Actor.K2_GetActorLocation` (`self.Get Locked On Actor`))))) (`Pawn.GetControlRotation` (`Actor.Instigator` (`self.GetOwner`)))))) (`GameplayStatics.GetWorldDeltaSeconds`)) -3.0 3.0))))