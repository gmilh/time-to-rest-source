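; Actor component that drives its owner's camera and spring arm from gameplay state: death, aiming, falling, combat or default.
; Each tick it picks the highest-priority configured state and interpolates FOV, arm length and socket offset toward it, snapping on BeginPlay.
; Arm length scales with viewport aspect ratio when the camera's ratio is unconstrained.
; Auto-rotation yaws the controller toward sideways movement, with a timed pause available for manual input.
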(event `self.ReceiveBeginPlay`
  (`self.Init Camera System`))

(event `self.ReceiveTick`
  (params (DeltaSeconds :type "Float (single-precision)"))
  (`self.Update Camera System`)
  (`self.Update Camera Rotation`))

(fn `Disable Auto Rotation`
  (set `self.Auto Rotation Enabled` false)
  (`KismetSystemLibrary.K2_SetTimerDelegate` (`|CreateDelegate` :!event `Enable Auto Rotation`) 0.2))

(fn `Enable Auto Rotation`
  (set `self.Auto Rotation Enabled` true))

(fn `Get Current Camera State`
  (returns (ReturnValue :type "/Game/Blueprints/Camera/E_CameraState Enum"))
  (return (select `bool` (and (`self.Get Is Dead`) (`BlueprintMapLibrary.Map_Contains` (`self.Camera Configurations`) "NewEnumerator6")) :`false` (select `bool` (and (`self.Is Aiming`) (`BlueprintMapLibrary.Map_Contains` (`self.Camera Configurations`) "NewEnumerator5")) :`false` (select `bool` (and (`self.Get Is Falling`) (`BlueprintMapLibrary.Map_Contains` (`self.Camera Configurations`) "NewEnumerator2")) :`false` (select `bool` (and (`self.In Combat`) (`BlueprintMapLibrary.Map_Contains` (`self.Camera Configurations`) "NewEnumerator7")) :`false` "NewEnumerator1" :`true` "NewEnumerator7" :!type "/Game/Blueprints/Camera/E_CameraState Enum") :`true` "NewEnumerator2") :`true` "NewEnumerator5") :`true` "NewEnumerator6")))

(fn `Get Is Dead`
  (returns (ReturnValue :type Boolean))
  (`self.Health`
    (:`then`
      (return (not (`/Game/Blueprints/Combat/Components/BP_HealthSystem.Get Has Remaining HP` (`self.Health`)))))
    (:`else`
      (return false))))

(fn `Get Is Falling`
  (returns (ReturnValue :type Boolean))
  (`self.Character Movement`
    (:`then`
      (return (`NavMovementComponent.IsFalling` (`self.Character Movement`))))
    (:`else`
      (return false))))

(fn `Init Additional Components`
  (if (`BlueprintMapLibrary.Map_Contains` (`self.Camera Configurations`) "NewEnumerator5")
    (set `self.Lock On Component` (`Actor.GetComponentByClass` (`self.GetOwner`) "/Game/Blueprints/Camera/BP_LockOnSystem.BP_LockOnSystem_C")))
  (if (`BlueprintMapLibrary.Map_Contains` (`self.Camera Configurations`) "NewEnumerator2")
    (bind _output_get (set `self.Character Movement` (`Actor.GetComponentByClass` (`self.GetOwner`) "/Script/Engine.CharacterMovementComponent")))
    (`/Engine/EditorBlueprintResources/StandardMacros.IsValid` _output_get
      (:`Is Valid`
        _)
      (:`Is Not Valid`
        (`KismetSystemLibrary.PrintString` (`KismetStringLibrary.Concat_StrStr` (`KismetSystemLibrary.GetDisplayName` (`self.GetOwner`)) " does not have the " "'Character Movement Component'" " required to handle a " "'Falling'" " camera state.") true true (struct :`G` 0.66 :`B` 1.0 :`A` 1.0) 8.0))))
  (if (`BlueprintMapLibrary.Map_Contains` (`self.Camera Configurations`) "NewEnumerator6")
    (bind _output_get_2 (set `self.Health` (`Actor.GetComponentByClass` (`self.GetOwner`) "/Game/Blueprints/Combat/Components/BP_HealthSystem.BP_HealthSystem_C")))
    (`/Engine/EditorBlueprintResources/StandardMacros.IsValid` _output_get_2
      (:`Is Not Valid`
        (bind _output_get_3 (set `self.Health` (`Actor.GetComponentByClass` (`Pawn.GetController` (`Actor.Instigator` (`self.GetOwner`))) "/Game/Blueprints/Combat/Components/BP_HealthSystem.BP_HealthSystem_C")))
        (`/Engine/EditorBlueprintResources/StandardMacros.IsValid` _output_get_3
          (:`Is Not Valid`
            (`KismetSystemLibrary.PrintString` (`KismetStringLibrary.Concat_StrStr` (`KismetSystemLibrary.GetDisplayName` (`self.GetOwner`)) " nor its controller have an " "'BP_HealthSystem' component" " required to handle a " "'Death'" " camera state.") true true (struct :`G` 0.66 :`B` 1.0 :`A` 1.0) 8.0)))))))

(fn `Init Camera System`
  (locals (`New Camera Parameters` :type "/Game/Blueprints/Camera/S_CameraValues Structure"))
  (bind (_value _returnvalue) (`BlueprintMapLibrary.Map_Find` (`self.Camera Configurations`) (`self.Get Current Camera State`)))
  (`self.Init Required Components`)
  (bind _output_get (set `local.New Camera Parameters` (select `bool` _returnvalue :`false` (make `/Game/Blueprints/Camera/S_CameraValues`) :`true` _value)))
  (bind _structout (setmembers `/Game/Blueprints/Camera/S_CameraValues` :`StructRef` _output_get :`Interpolation Speed` 0.0)) ; Override Interpolation speed so the camera instantly\nshift to the new parameters given
  (set `local.New Camera Parameters` _structout)
  (`self.Update Camera Component` (`local.New Camera Parameters`))
  (`self.Update Camera Arm Component` (`local.New Camera Parameters`)))

(fn `Init Required Components`
  (`self.Init Target Components`)
  (`self.Init Additional Components`))

(fn `Init Target Components`
  (set `self.Camera Target` (`Actor.GetComponentByClass` (`self.GetOwner`) "/Script/Engine.CameraComponent"))
  (for _array_element (`Actor.K2_GetComponentsByClass` (`self.GetOwner`) "/Script/Engine.SpringArmComponent")
    (if (== _array_element (`SceneComponent.GetAttachParent` (`self.Camera Target`)))
      (set `self.SpringArm Target` _array_element)
      (break))))

(fn `Scale Arm Lenght by Viewport Ratio`
  (params (A :type "Float (double-precision)"))
  (returns (ReturnValue :type "Float (double-precision)"))
  (bind (_x _y) (`KismetMathLibrary.BreakVector2D` (`WidgetLayoutLibrary.GetViewportSize`)))
  (return (* A (`KismetMathLibrary.SelectFloat` 1.0 (`KismetMathLibrary.MapRangeUnclamped` (/ _x _y) (`CameraComponent.AspectRatio` (`self.Camera Target`)) 2.388889 1.0 1.3125) (`CameraComponent.bConstrainAspectRatio` (`self.Camera Target`))))))

(fn `Set In Combat`
  (params (`New Value` :type Boolean))
  (set `self.In Combat` `New Value`))

(fn `Set Is Aiming`
  (params (`New Value` :type Boolean))
  (bind _output_get (set `self.Is Aiming` `New Value`))
  (`self.On Aiming State Change` _output_get))

(fn `Update Camera Arm Component`
  (params (`New Parameters` :type "/Game/Blueprints/Camera/S_CameraValues Structure"))
  (locals (`New Camera Parameters` :type "/Game/Blueprints/Camera/S_CameraValues Structure"))
  (bind ((`ArmSocketOffset_14_250B4D69433AD5CBF1D113A3691B7187` _armsocketoffset) (`InterpolationSpeed_13_EA6EE996401EEBF703DA778184B31450` _interpolationspeed)) (break `/Game/Blueprints/Camera/S_CameraValues` (`local.New Camera Parameters`)))
  (set `local.New Camera Parameters` `New Parameters`)
  (`self.SpringArm Target`
    (:`then`
      (set `SpringArmComponent.TargetArmLength` (`KismetMathLibrary.FInterpTo` (`SpringArmComponent.TargetArmLength` (`self.SpringArm Target`)) (`self.Scale Arm Lenght by Viewport Ratio` (`.ArmLenght_9_437FEAD749E6B1550C16CA830BD20107` (break `/Game/Blueprints/Camera/S_CameraValues` (`local.New Camera Parameters`)))) (`GameplayStatics.GetWorldDeltaSeconds`) (`.InterpolationSpeed_13_EA6EE996401EEBF703DA778184B31450` (break `/Game/Blueprints/Camera/S_CameraValues` (`local.New Camera Parameters`)))) (`self.SpringArm Target`))
      (set `SpringArmComponent.SocketOffset` (`KismetMathLibrary.VInterpTo` (`SpringArmComponent.SocketOffset` (`self.SpringArm Target`)) _armsocketoffset (`GameplayStatics.GetWorldDeltaSeconds`) _interpolationspeed) (`self.SpringArm Target`)))
    (:`else`)))

(fn `Update Camera Component`
  (params (`New Parameters` :type "/Game/Blueprints/Camera/S_CameraValues Structure"))
  (locals (`New Camera Parameters` :type "/Game/Blueprints/Camera/S_CameraValues Structure"))
  (bind ((`FieldofView_10_48E21ED24B8236090500979CD345B39C` _fieldofview) (`InterpolationSpeed_13_EA6EE996401EEBF703DA778184B31450` _interpolationspeed)) (break `/Game/Blueprints/Camera/S_CameraValues` (`local.New Camera Parameters`)))
  (set `local.New Camera Parameters` `New Parameters`)
  (`self.Camera Target`
    (:`then`
      (`CameraComponent.SetFieldOfView` (`self.Camera Target`) (`KismetMathLibrary.FInterpTo` (`CameraComponent.FieldOfView` (`self.Camera Target`)) _fieldofview (`GameplayStatics.GetWorldDeltaSeconds`) _interpolationspeed)))
    (:`else`)))

(fn `Update Camera Rotation`
  (bind _turn_rate (`self.Turn Rate`))
  ;[1 1 1] Can be disabled calling 'Disable Auto Rotation' when manual camera input is being given
  (if (`self.Auto Rotation Enabled`)
    (`Pawn.AddControllerYawInput` (`Actor.Instigator` (`self.GetOwner`)) (* (`KismetMathLibrary.Dot_VectorVector` (`KismetMathLibrary.GetRightVector` (`KismetMathLibrary.MakeRotator` 0.0 0.0 (.yaw (`Pawn.GetControlRotation` (`Actor.Instigator` (`self.GetOwner`)))))) (`MovementComponent.Velocity` (`self.Character Movement`))) (`KismetMathLibrary.FClamp` (`KismetMathLibrary.Dot_VectorVector` (`Actor.GetActorForwardVector` (`self.GetOwner`)) (`MovementComponent.Velocity` (`self.Character Movement`)))) (`KismetMathLibrary.SelectFloat` _turn_rate (* _turn_rate (`self.Air Turn Rate Multplier`)) (`NavMovementComponent.IsMovingOnGround` (`self.Character Movement`))) (`GameplayStatics.GetWorldDeltaSeconds`)))))

(fn `Update Camera System`
  (locals (`New Camera Parameters` :type "/Game/Blueprints/Camera/S_CameraValues Structure"))
  (bind (_value _returnvalue) (`BlueprintMapLibrary.Map_Find` (`self.Camera Configurations`) (`self.Get Current Camera State`)))
  (set `local.New Camera Parameters` (select `bool` _returnvalue :`false` (make `/Game/Blueprints/Camera/S_CameraValues`) :`true` _value))
  (`self.Update Camera Component` (`local.New Camera Parameters`))
  (`self.Update Camera Arm Component` (`local.New Camera Parameters`)))