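; Base character Blueprint that provides a timed, coloured emissive damage flash on the character mesh.
; On BeginPlay it creates and caches dynamic material instances for every Mesh material slot.
; PlayDamageFlashing sets the emissive colour on those materials, fits the DamageFlashing timeline to the given duration and restarts it.
; The timeline drives emissive intensity, then resets the colour to white when finished playing forward.
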(event `self.ReceiveBeginPlay`
  (`self.Init Dynamic Materials`))

(fn `Init Dynamic Materials`
  (`KismetArrayLibrary.Array_Clear` (`self.Character Materials`))
  (for _array_element (`|MakeArray` (`self.Mesh`))
    (for _index (range (+ (`KismetArrayLibrary.Array_LastIndex` (`MeshComponent.GetMaterials` _array_element)) 1))
      (bind _returnvalue (`PrimitiveComponent.CreateDynamicMaterialInstance` _array_element _index null "None"))
      (`KismetArrayLibrary.Array_Add` (`self.Character Materials`) _returnvalue))))

(fn `Play Damage Flashing`
  (params (Duration :type "Float (double-precision)") (Colour :type "LinearColor Structure"))
  (locals (`Target Colour` :type "LinearColor Structure" :default (struct :`R` 1.0 :`A` 1.0)) (`Target Duration` :type "Float (double-precision)" :default 0.2))
  (set `local.Target Duration` Duration)
  (set `local.Target Colour` Colour)
  (for _array_element (`self.Character Materials`)
    (`MaterialInstanceDynamic.SetVectorParameterValue` _array_element "Emissive Colour" (`local.Target Colour`)))
  (`/Game/Blueprints/Libraries/BPLib_CustomFunctions.Set Timeline Duration` (`self.Damage Flashing`) (`local.Target Duration`))
  (`TimelineComponent.PlayFromStart` (`self.Damage Flashing`)))

(fn `UserConstructionScript`)