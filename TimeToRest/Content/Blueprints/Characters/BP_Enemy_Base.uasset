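; Base melee enemy character that fights, reacts to damage, dies and randomizes its mesh and skin on construction.
; MeleeCombatSystem picks combo attack objects and tracks state, with behaviour-tree-triggered montages and anim notifies opening and closing weapon damage.
; HealthSystem updates drive flashing, death, and hurt montages that set blackboard "Stunned", skipping stagger during active damage frames.
; PawnSensing writes seen pawns to the blackboard, and damage types supply impact effects.
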(event `self.ReceiveBeginPlay`
  (`parent.ReceiveBeginPlay`))

(event `/Game/Blueprints/Combat/Interfaces/BPI_LockOnTarget.Set Is Targeted`
  (params (`Is Target` :type Boolean))
  (`SceneComponent.SetHiddenInGame` (`self.Billboard`) (not `Is Target`) false))

(event `self.Initiate Melee Attack`
  (params (`Attack Class` :type "/Game/Blueprints/Combat/AttackClasses/BP_Attack_Base Class Reference"))
  (bind _current_state (`/Game/Blueprints/Combat/Components/BP_MeleeCombatSystem.Get Current State` (`self.Melee Combat System`)))
  (switch `/Game/Blueprints/Combat/E_MeleeState` _current_state
    (:`NewEnumerator0`
      (bind (_success _current_attack) (`/Game/Blueprints/Combat/Components/BP_MeleeCombatSystem.Get Next Attack in Combo` (`self.Melee Combat System`)))
      ;[1 1 1 1 56] Initiate an Attack
      ;;[1 1 1] Use the Actor Component BP_EnemyAttack, which handles combo and cooldown,
      ;; to get a class of what the next attack would be
      (bind _returnvalue (`|GenericCreateObject` _current_attack self))
      (set `self.Current Attack` _returnvalue)
      (`self.PlayAnimMontage` (`/Game/Blueprints/Combat/AttackClasses/BP_Attack_Base.Animation` (`self.Current Attack`)))
      (`/Game/Blueprints/Combat/Components/BP_MeleeCombatSystem.Set Melee State` (`self.Melee Combat System`) "NewEnumerator1"))))

(event `self.Execute Melee Attack Damage`
  ;[1 1 1 1 56] Execute Attack - Begin Damaging Frames
  (bind _current_attack (`self.Current Attack`)
    (:`then`
      (message `/Game/Blueprints/Combat/Weapons/Melee/BPI_MeleeWeapon.Initiate Dealing Damage` (`ChildActorComponent.ChildActor` (`self.Melee Weapon`)) (`/Game/Blueprints/Combat/AttackClasses/BP_Attack_Base.Damage` _current_attack))
      (`/Game/Blueprints/Combat/Components/BP_MeleeCombatSystem.Set Melee State` (`self.Melee Combat System`) "NewEnumerator4"))
    (:`else`)))

(event `self.Terminate Current Melee Attack`
  ;[1 1 1 1 56] End Current Attack and Damage Frames
  (message `/Game/Blueprints/Combat/Weapons/Melee/BPI_MeleeWeapon.Terminate Dealing Damage` (`ChildActorComponent.ChildActor` (`self.Melee Weapon`)))
  (set `self.Current Attack` null) ; Because Current Attack is an object and not an actor,\nsimply setting the reference to null will also result in\nthe object being cleared from memory
  (`/Game/Blueprints/Combat/Components/BP_MeleeCombatSystem.Set Melee State` (`self.Melee Combat System`) "NewEnumerator0"))

(event `self.ReceiveAnyDamage`
  (params (Damage :type "Float (single-precision)") (DamageType :type "DamageType Object Reference") (InstigatedBy :type "Controller Object Reference") (DamageCauser :type "Actor Object Reference"))
  (`/Game/Blueprints/Combat/Components/BP_HealthSystem.Decrement HP` (`self.Health System`) Damage)
  (`GameplayStatics.PlaySoundAtLocation` "/Game/Audio/SC_DeathBlow.SC_DeathBlow" (`self.K2_GetActorLocation`) (struct) 1.0 1.0 0.0 null null null))

(event `self.Health System.On HP Amount Update`
  (params (`HP Percent` :type "Float (single-precision)"))
  (bind _capsulecomponent (`self.CapsuleComponent`))
  (if (<= `HP Percent` 0.0)
    (set `self.bCanBeDamaged` false)
    (`self.Play Damage Flashing` 0.8 (struct :`R` 1.0 :`A` 1.0))
    (`PrimitiveComponent.SetCollisionResponseToAllChannels` _capsulecomponent "ECR_Ignore")
    (`PrimitiveComponent.SetCollisionResponseToChannel` _capsulecomponent "ECC_WorldStatic" "ECR_Block")
    (`self.Terminate Current Melee Attack`)
    (`BlackboardComponent.SetValueAsBool` (`AIBlueprintHelperLibrary.GetBlackboard` (`self.GetController`)) "Stunned" true)
    (bind _returnvalue (`self.GetCurrentMontage`))
    (`self.StopAnimMontage` _returnvalue)
    (`|ExecutionSequence`
      (:`then_0`
        (goto _label :!via `Close`))
      (:`then_1`
        (bind _returnvalue_2 (`self.PlayAnimMontage` "/Game/Animations/WarriorZombie/AM_Death_Brute.AM_Death_Brute"))
        (`KismetSystemLibrary.Delay` _returnvalue_2)
        (`self.K2_DestroyActor`)))
    (else
      (`self.Play Damage Flashing` 0.14 (struct :`R` 0.333333 :`G` 0.333333 :`A` 1.0))
      (if (not (`BlackboardComponent.GetValueAsBool` (`AIBlueprintHelperLibrary.GetBlackboard` (`self.GetController`)) "Stunned"))
        (bind _current_state (`/Game/Blueprints/Combat/Components/BP_MeleeCombatSystem.Get Current State` (`self.Melee Combat System`)))
        (switch `/Game/Blueprints/Combat/E_MeleeState` _current_state
          (:`NewEnumerator0`
            _)
          (:`NewEnumerator1`
            _)
          (:`NewEnumerator5`
            _))
        (`self.Terminate Current Melee Attack`)
        (`BlackboardComponent.SetValueAsBool` (`AIBlueprintHelperLibrary.GetBlackboard` (`self.GetController`)) "Stunned" true)
        (bind _returnvalue_3 (`self.GetCurrentMontage`))
        (`self.StopAnimMontage` _returnvalue_3)
        (bind _returnvalue_4 (`self.PlayAnimMontage` "/Game/Animations/WarriorZombie/AM_Hurt_Brute.AM_Hurt_Brute"))
        (`KismetSystemLibrary.RetriggerableDelay` _returnvalue_4)
        (`/Engine/EditorBlueprintResources/StandardMacros.Gate` false :!label _label
          (:`Exit`
            (`BlackboardComponent.SetValueAsBool` (`AIBlueprintHelperLibrary.GetBlackboard` (`self.GetController`)) "Stunned" false)))))))

(event `self.ReceivePointDamage`
  (params (Damage :type "Float (single-precision)") (DamageType :type "DamageType Object Reference") (HitLocation :type "Vector Structure") (HitNormal :type "Vector Structure") (HitComponent :type "PrimitiveComponent Object Reference") (BoneName :type Name) (ShotFromDirection :type "Vector Structure") (InstigatedBy :type "Controller Object Reference") (DamageCauser :type "Actor Object Reference") (HitInfo :type "HitResult Structure (by ref)"))
  (bind (_bblockinghit _binitialoverlap _time _distance _location _impactpoint) (`GameplayStatics.BreakHitResult` HitInfo))
  (bind (_particle_effects _sound_effects) (message `/Game/Blueprints/Combat/DamageClasses/BPI_Damage.Get Spatial Feedback` DamageType))
  (for _array_element _particle_effects
    (`GameplayStatics.SpawnEmitterAtLocation` _array_element _impactpoint))
  (for _array_element_2 _sound_effects
    (`GameplayStatics.SpawnSoundAtLocation` _array_element_2 _impactpoint (struct) 1.0 1.0 0.0 null null)))

(event `self.PawnSensing.OnSeePawn`
  (params (Pawn :type "Pawn Object Reference"))
  (`BlackboardComponent.SetValueAsObject` (`AIBlueprintHelperLibrary.GetBlackboard` (`self.GetController`)) "Engaged Pawn" Pawn))

(event `self.PawnSensing.OnHearNoise`
  (params (Instigator :type "Pawn Object Reference") (Location :type "Vector Structure (by ref)") (Volume :type "Float (single-precision)")))

(fn `UserConstructionScript`
  (locals (Skin :type "MaterialInterface Object Reference"))
  (`SkinnedMeshComponent.SetSkinnedAssetAndUpdate` (`self.Mesh`) (select `bool` (`KismetMathLibrary.RandomBoolWithWeight` 0.4) :`false` "/Game/SK_Meshes/WarriorZombie/Helmet_Warrior_RM.Helmet_Warrior_RM" :`true` "/Game/SK_Meshes/WarriorZombie/Helmet_Warrior_Var01_RM.Helmet_Warrior_Var01_RM" :!type "SkeletalMesh Object Reference") true)
  (set `local.Skin` (select `bool` (`KismetMathLibrary.RandomBoolWithWeight` 0.5) :`false` "/Game/Materials/Characters/WarriorZombie/MI_Body_2.MI_Body_2" :`true` "/Game/Materials/Characters/WarriorZombie/MI_Body_3.MI_Body_3" :!type "MaterialInterface Object Reference"))
  (for _index (range 3)
    (`PrimitiveComponent.SetMaterial` (`self.Mesh`) _index (`local.Skin`)))
  (`parent.UserConstructionScript`))