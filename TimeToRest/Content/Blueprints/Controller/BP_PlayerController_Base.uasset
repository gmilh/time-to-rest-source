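; Base player controller that creates the player's health bar widget and tracks whether the player is using a gamepad.
; HealthSystem HP updates feed the health bar's percentage.
; Any key press checks for gamepad input and passes the result to the GameInstance and HUD.
; On possess it binds to the pawn's destruction; pawn-destroyed and damage-instigated handlers are empty, and force feedback and camera shake nodes are unconnected.
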(event `self.ReceiveBeginPlay`
  (bind _returnvalue (`|CreateWidget` "/Game/Blueprints/UI/WBP_HealthBar.WBP_HealthBar_C" self))
  (bind _output_get (set `self.Health bar` _returnvalue))
  (`UserWidget.AddToPlayerScreen` _output_get 0))

(event `self.ReceivePossess`
  (params (PossessedPawn :type "Pawn Object Reference"))
  (add `self.OnDestroyed` (`self.K2_GetPawn`) (`|CreateDelegate` :!event `Pawn Destroyed`)))

(event `Key|AnyKey` :consume false :overrideparent false
  (params (Key :type "Key Structure"))
  (bind _returnvalue (`KismetInputLibrary.Key_IsGamepadKey` Key))
  (:`Pressed`
    (message `/Game/Blueprints/Game/BPI_InputDeviceData.Set Using Gamepad` (`GameplayStatics.GetGameInstance`) _returnvalue)
    (message `/Game/Blueprints/UI/BPI_HUD.Set Gamepad Input` (`self.GetHUD`) _returnvalue)))

(event `Pawn Destroyed`
  (params (DestroyedActor :type "Actor Object Reference")))

(event `self.ReceiveInstigatedAnyDamage`
  (params (Damage :type "Float (single-precision)") (DamageType :type "DamageType Object Reference") (DamagedActor :type "Actor Object Reference") (DamageCauser :type "Actor Object Reference")))

(event `self.Health System.On HP Amount Update`
  (params (`HP Percent` :type "Float (single-precision)"))
  (set `/Game/Blueprints/UI/WBP_HealthBar.Current HP` `HP Percent` (`self.Health bar`)))

(fn `UserConstructionScript`)